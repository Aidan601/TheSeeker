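; SlenderMode sets up a Slender-style paper hunt on BeginPlay, playing a flashlight click and setting an eight-paper counter.
; It randomizes pre-placed Paper actors by culling rather than spawning, using a shuffled boolean array over ten location tags.
; Selected tags get their papers shuffled and trimmed by PaperIn, with Boil always selected.
; A final pass clears any tag still holding exactly four papers.
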(event `self.ReceiveBeginPlay`
  (bind _false (`self.False`))
  (bind _true (`self.True`))
  (bind _array (`|MakeArray` _false _false _true _true _true _true _true _true _true _true))
  (`GameplayStatics.PlaySoundAtLocation` "/Game/Sound/flashlightclick_Cue.flashlightclick_Cue" (`self.K2_GetActorLocation`) (struct) 1.0 1.0 0.0 null null null)
  (bind _output_get (set `self.Paper Left` 8))
  (set `self.Paper Total` _output_get)
  (`KismetArrayLibrary.Array_Shuffle` _array)
  (for _index (range (+ (`KismetArrayLibrary.Array_Length` _array) 1))
    (if (== 0 _index)
      (bind _output (`|GetArrayItem` _array _index))
      (if _output
        (bind _outactors (`GameplayStatics.GetAllActorsOfClassWithTag` "/Game/Blueprints/Paper.Paper_C" "Silo"))
        (`KismetArrayLibrary.Array_Shuffle` _outactors)
        (for _index_2 (range (+ (- (`KismetArrayLibrary.Array_Length` _outactors) (+ (`self.Paper In`) 1)) 1))
          (`self.K2_DestroyActor` (`|GetArrayItem` _outactors _index_2))))
      (elif (== 1 _index)
        (if _output
          (bind _outactors_2 (`GameplayStatics.GetAllActorsOfClassWithTag` "/Game/Blueprints/Paper.Paper_C" "Rocks"))
          (`KismetArrayLibrary.Array_Shuffle` _outactors_2)
          (for _index_3 (range (+ (- (`KismetArrayLibrary.Array_Length` _outactors_2) (+ (`self.Paper In`) 1)) 1))
            (`self.K2_DestroyActor` (`|GetArrayItem` _outactors_2 _index_3))))
        (elif (== 2 _index)
          (if _output
            (bind _outactors_3 (`GameplayStatics.GetAllActorsOfClassWithTag` "/Game/Blueprints/Paper.Paper_C" "Walls"))
            (`KismetArrayLibrary.Array_Shuffle` _outactors_3)
            (for _index_4 (range (+ (- (`KismetArrayLibrary.Array_Length` _outactors_3) (+ (`self.Paper In`) 1)) 1))
              (`self.K2_DestroyActor` (`|GetArrayItem` _outactors_3 _index_4))))
          (elif (== 3 _index)
            (if _output
              (bind _outactors_4 (`GameplayStatics.GetAllActorsOfClassWithTag` "/Game/Blueprints/Paper.Paper_C" "Wood"))
              (`KismetArrayLibrary.Array_Shuffle` _outactors_4)
              (for _index_5 (range (+ (- (`KismetArrayLibrary.Array_Length` _outactors_4) (+ (`self.Paper In`) 1)) 1))
                (`self.K2_DestroyActor` (`|GetArrayItem` _outactors_4 _index_5))))
            (elif (== 4 _index)
              (if _output
                (bind _outactors_5 (`GameplayStatics.GetAllActorsOfClassWithTag` "/Game/Blueprints/Paper.Paper_C" "Tunnel"))
                (`KismetArrayLibrary.Array_Shuffle` _outactors_5)
                (for _index_6 (range (+ (- (`KismetArrayLibrary.Array_Length` _outactors_5) (+ (`self.Paper In`) 1)) 1))
                  (`self.K2_DestroyActor` (`|GetArrayItem` _outactors_5 _index_6))))
              (elif (== 5 _index)
                (if _output
                  (bind _outactors_6 (`GameplayStatics.GetAllActorsOfClassWithTag` "/Game/Blueprints/Paper.Paper_C" "Truck"))
                  (`KismetArrayLibrary.Array_Shuffle` _outactors_6)
                  (for _index_7 (range (+ (- (`KismetArrayLibrary.Array_Length` _outactors_6) (+ (`self.Paper In`) 1)) 1))
                    (`self.K2_DestroyActor` (`|GetArrayItem` _outactors_6 _index_7))))
                (elif (== 6 _index)
                  (if _output
                    (bind _outactors_7 (`GameplayStatics.GetAllActorsOfClassWithTag` "/Game/Blueprints/Paper.Paper_C" "Trucks"))
                    (`KismetArrayLibrary.Array_Shuffle` _outactors_7)
                    (for _index_8 (range (+ (- (`KismetArrayLibrary.Array_Length` _outactors_7) (+ (`self.Paper In`) 1)) 1))
                      (`self.K2_DestroyActor` (`|GetArrayItem` _outactors_7 _index_8))))
                  (elif (== 7 _index)
                    (if _output
                      (bind _outactors_8 (`GameplayStatics.GetAllActorsOfClassWithTag` "/Game/Blueprints/Paper.Paper_C" "Tree"))
                      (`KismetArrayLibrary.Array_Shuffle` _outactors_8)
                      (for _index_9 (range (+ (- (`KismetArrayLibrary.Array_Length` _outactors_8) (+ (`self.Paper In`) 1)) 1))
                        (`self.K2_DestroyActor` (`|GetArrayItem` _outactors_8 _index_9))))
                    (elif (== 8 _index)
                      (if _output
                        (bind _outactors_9 (`GameplayStatics.GetAllActorsOfClassWithTag` "/Game/Blueprints/Paper.Paper_C" "Bathroom"))
                        (`KismetArrayLibrary.Array_Shuffle` _outactors_9)
                        (for _index_10 (range (+ (- (`KismetArrayLibrary.Array_Length` _outactors_9) (+ (`self.Paper In`) 1)) 1))
                          (`self.K2_DestroyActor` (`|GetArrayItem` _outactors_9 _index_10))))
                      (elif (== 9 _index)
                        (if true
                          (bind _outactors_10 (`GameplayStatics.GetAllActorsOfClassWithTag` "/Game/Blueprints/Paper.Paper_C" "Boil"))
                          (`KismetArrayLibrary.Array_Shuffle` _outactors_10)
                          (for _index_11 (range (+ (- (`KismetArrayLibrary.Array_Length` _outactors_10) (+ (`self.Paper In`) 1)) 1))
                            (`self.K2_DestroyActor` (`|GetArrayItem` _outactors_10 _index_11)))))))))))))))
  (bind _outactors_11 (`GameplayStatics.GetAllActorsOfClassWithTag` "/Game/Blueprints/Paper.Paper_C" "Silo"))
  (if (== 4 (`KismetArrayLibrary.Array_Length` _outactors_11))
    (`self.K2_DestroyActor` _outactors_11))
  (bind _outactors_12 (`GameplayStatics.GetAllActorsOfClassWithTag` "/Game/Blueprints/Paper.Paper_C" "Rocks"))
  (if (== 4 (`KismetArrayLibrary.Array_Length` _outactors_12))
    (`self.K2_DestroyActor` _outactors_12))
  (bind _outactors_13 (`GameplayStatics.GetAllActorsOfClassWithTag` "/Game/Blueprints/Paper.Paper_C" "Walls"))
  (if (== 4 (`KismetArrayLibrary.Array_Length` _outactors_13))
    (`self.K2_DestroyActor` _outactors_13))
  (bind _outactors_14 (`GameplayStatics.GetAllActorsOfClassWithTag` "/Game/Blueprints/Paper.Paper_C" "Wood"))
  (if (== 4 (`KismetArrayLibrary.Array_Length` _outactors_14))
    (`self.K2_DestroyActor` _outactors_14))
  (bind _outactors_15 (`GameplayStatics.GetAllActorsOfClassWithTag` "/Game/Blueprints/Paper.Paper_C" "Tunnel"))
  (if (== 4 (`KismetArrayLibrary.Array_Length` _outactors_15))
    (`self.K2_DestroyActor` _outactors_15))
  (bind _outactors_16 (`GameplayStatics.GetAllActorsOfClassWithTag` "/Game/Blueprints/Paper.Paper_C" "Truck"))
  (if (== 4 (`KismetArrayLibrary.Array_Length` _outactors_16))
    (`self.K2_DestroyActor` _outactors_16))
  (bind _outactors_17 (`GameplayStatics.GetAllActorsOfClassWithTag` "/Game/Blueprints/Paper.Paper_C" "Trucks"))
  (if (== 4 (`KismetArrayLibrary.Array_Length` _outactors_17))
    (`self.K2_DestroyActor` _outactors_17))
  (bind _outactors_18 (`GameplayStatics.GetAllActorsOfClassWithTag` "/Game/Blueprints/Paper.Paper_C" "Tree"))
  (if (== 4 (`KismetArrayLibrary.Array_Length` _outactors_18))
    (`self.K2_DestroyActor` _outactors_18))
  (bind _outactors_19 (`GameplayStatics.GetAllActorsOfClassWithTag` "/Game/Blueprints/Paper.Paper_C" "Bathroom"))
  (if (== 4 (`KismetArrayLibrary.Array_Length` _outactors_19))
    (`self.K2_DestroyActor` _outactors_19))
  (bind _outactors_20 (`GameplayStatics.GetAllActorsOfClassWithTag` "/Game/Blueprints/Paper.Paper_C" "Boil"))
  (if (== 4 (`KismetArrayLibrary.Array_Length` _outactors_20))
    (`self.K2_DestroyActor` _outactors_20)))

(fn `UserConstructionScript`)