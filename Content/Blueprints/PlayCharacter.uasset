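; Player character Blueprint handling movement, mouse look, sprinting and a flashlight that F or right mouse toggles with a click sound.
; Left Shift sprints when Stamina allows, changing walk speed, spring arm pitch and footstep interval; Stamina is only read here.
; Movement input traces downward for the surface type to pick tile or default footstep sounds, played on a looping timer while moving horizontally and reset on sprint changes.
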(event `Key|F`
  (params (Key :type "Key Structure"))
  (bind _flashlight (`self.FlashLight`))
  ;[1 1 1] Flashlight
  (:`Pressed`
    (`GameplayStatics.PlaySoundAtLocation` "/Game/Sound/flashlightclick_Cue.flashlightclick_Cue" (`self.K2_GetActorLocation`) (struct) 1.0 1.0 0.0 null null null :!label _label)
    (`/Engine/EditorBlueprintResources/StandardMacros.FlipFlop`
      (:`A`
        (`SceneComponent.SetVisibility` _flashlight false false))
      (:`B`
        (`SceneComponent.SetVisibility` _flashlight true false)))))

(event `InputAxis|LookX`
  (params (AxisValue :type "Float (single-precision)"))
  ;[1 1 1] Look
  (`self.AddControllerYawInput` AxisValue))

(event `InputAxis|LookY`
  (params (AxisValue :type "Float (single-precision)"))
  ;[1 1 1] Look
  (`self.AddControllerPitchInput` AxisValue))

(event `Key|RightMouseButton`
  (params (Key :type "Key Structure"))
  ;[1 1 1] Flashlight
  (:`Pressed`
    (goto _label)))

(event `Key|LeftShift`
  (params (Key :type "Key Structure"))
  ;[1 1 1] Sprint
  (:`Pressed`
    (if (>= (`self.Stamina`) 1)
      (set `self.IsSprinting?` true)
      (set `CharacterMovementComponent.MaxWalkSpeed` 2000.0 (`self.CharacterMovement`))
      (`SceneComponent.K2_SetRelativeRotation` (`self.SpringArm`) (`KismetMathLibrary.MakeRotator` 0.0 -25.0) false false)
      (set `self.Footstep Int` 0.4)
      (`self.ResetFootstep` :!label _label_2)))
  (:`Released`
    (set `CharacterMovementComponent.MaxWalkSpeed` 200.0 (`self.CharacterMovement`))
    (set `self.IsSprinting?` false)
    (`SceneComponent.K2_SetRelativeRotation` (`self.SpringArm`) (`KismetMathLibrary.MakeRotator` 0.0) false false)
    (set `self.Footstep Int` 0.5)
    (goto _label_2)))

(event `InputAxis|MoveRight`
  (params (AxisValue :type "Float (single-precision)"))
  (bind (_returnvalue_x _returnvalue_y _returnvalue_z) (`KismetMathLibrary.BreakVector` (`self.GetVelocity`)))
  ;[1 1 1] Movement
  (`self.AddMovementInput` (`SceneComponent.GetRightVector` (`self.Camera`)) AxisValue)
  (`self.CheckPhysicsMaterial` :!label _label_3)
  ;[1 1 1] Footstep Noise
  (if (and (or (> _returnvalue_x 0.1) (< _returnvalue_x -0.1) (> _returnvalue_y 0.1) (< _returnvalue_y -0.1)) (== _returnvalue_z 0.0))
    (`/Engine/EditorBlueprintResources/StandardMacros.DoOnce` false :!label _label_4
      (:`Completed`
        (bind _returnvalue (`KismetSystemLibrary.K2_SetTimerDelegate` (delegate `PlayFootstepSound`) (`self.Footstep Int`) true))))
    (else
      (`KismetSystemLibrary.K2_ClearAndInvalidateTimerHandle` _returnvalue :!label _label_5)
      (goto _label_4 :!via `Reset`))))

(event `InputAxis|MoveForward`
  (params (AxisValue :type "Float (single-precision)"))
  ;[1 1 1] Movement
  (`self.AddMovementInput` (`SceneComponent.GetForwardVector` (`self.Camera`)) AxisValue)
  (goto _label_3))

(event `PlayFootstepSound`
  ;[1 1 1] Footstep Noise
  (`GameplayStatics.PlaySoundAtLocation` (`self.Footstep SFX`) (- (`self.K2_GetActorLocation`) (0.0 0.0 44.0)) (struct) 1.0 1.0 0.0 null null null))

(event `ResetFootstep`
  ;[1 1 1] Footstep Noise
  (goto _label_5))

(event `CheckPhysicsMaterial`
  (bind _returnvalue (`self.K2_GetActorLocation`))
  ;[1 1 1] Checks Surface for Footsteps
  (bind (_outhit _returnvalue_2) (`KismetSystemLibrary.LineTraceSingle` _returnvalue (- _returnvalue (0.0 0.0 144.0)) "TraceTypeQuery1"))
  (if _returnvalue_2
    (switch `EPhysicalSurface` (`GameplayStatics.GetSurfaceType` _outhit)
      (:`SurfaceType_Default`
        (set `self.Footstep SFX` "/Game/Sound/Steps/Footsteps.Footsteps" :!label _label_6))
      (:`SurfaceType1`
        (goto _label_6))
      (:`SurfaceType2`
        (set `self.Footstep SFX` "/Game/Sound/Steps/Tile_Footsteps.Tile_Footsteps")))))

(fn `UserConstructionScript`)